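; GA_FireWeapon is a Gameplay Ability that fires a hitscan shot along the owning actor's forward vector.
; On activation it line-traces for Pawn objects from the owner's location out to RayTraceRange, ignoring the owner and drawing debug lines.
; A hit BP_ThirdPersonCharacter receives GE_Damage through its own AbilitySystemComponent, which serves as both source and target.
; A Sequence node then ends the ability, hit or miss.
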(event Ability|EventActivateAbility
  (bind _returnvalue (Ability|GetActorInfo))
  (bind _raytracerange (Variables|Default|GetRayTraceRange))
  (bind _owneractor (Utilities|Struct|BreakGameplayAbilityActorInfo _returnvalue))
  (bind _returnvalue_2 (Transformation|GetActorLocation _owneractor))
  (bind _returnvalue_3 (Transformation|GetActorRotation _owneractor))
  (bind _returnvalue_4 (Math|Vector|GetForwardVector _returnvalue_3))
  (bind _returnvalue_5 (* _returnvalue_4 _raytracerange))
  (bind _returnvalue_6 (+ _returnvalue_2 _returnvalue_5))
  (Utilities|FlowControl|Sequence
    (:then_0
      (bind (_outhit _returnvalue_7) (Collision|LineTraceForObjects _returnvalue_2 _returnvalue_6 (Utilities|Array|MakeArray "ObjectTypeQuery3") false (Utilities|Array|MakeArray _owneractor) "ForDuration"))
      (Rendering|Debug|DrawDebugLine _returnvalue_2 _returnvalue_6 "(R=1.000000,G=0.000000,B=0.000000,A=1.000000)" 1.0 5.0)
      (if _returnvalue_7
        (bind _asbp_third_person_character (Utilities|Casting|CastToBP_ThirdPersonCharacter (.HitActor (Collision|BreakHitResult _outhit))))
        (GameplayEffects|ApplyGameplayEffectToTarget :self (Variables|/Script/GAS.GASCharacter|GetAbilitySystemComponent _asbp_third_person_character) :GameplayEffectClass "/Game/Abilities/GE_Damage.GE_Damage_C" :Target (Variables|/Script/GAS.GASCharacter|GetAbilitySystemComponent _asbp_third_person_character) :Level 1.0)))
    (:then_1
      (Ability|EndAbility))))